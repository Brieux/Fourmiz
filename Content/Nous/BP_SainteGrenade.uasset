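; Holy grenade actor that bounces audibly on voxel terrain and explodes five seconds after spawning.
; The blast plays sounds, shakes the player camera and carves a large random-radius sphere from the VoxelWorld.
; It scatters short-lived, voxel-colored physics cubes and runs voxel physics through a cube part spawner.
; Finally it calls DestroyActor, then Explosion, which spawns Niagara and adds an overlap sphere messaging BPI_Destructible actors to destroy themselves.
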(event `self.ReceiveBeginPlay`
  (bind _returnvalue (`self.K2_GetActorLocation`))
  (bind _returnvalue_2 (`KismetMathLibrary.RandomFloatInRange` 1350.0 1500.0))
  (bind _world (`self.World`))
  (bind _world_2 (`self.World`))
  (bind _returnvalue_3 (`GameplayStatics.GetActorOfClass` "/Script/Voxel.VoxelWorld"))
  (set `self.World` _returnvalue_3)
  (bind _returnvalue_4 (`|GenericCreateObject` self "/Script/Voxel.VoxelPhysicsPartSpawner_Cubes"))
  (bind _output_get (set `self.NewVar` _returnvalue_4))
  (set `VoxelPhysicsPartSpawner_Cubes.Material` "/Voxel/Examples/Materials/RGB/M_VoxelMaterial_Colors_Parameter.M_VoxelMaterial_Colors_Parameter" _output_get)
  (set `VoxelPhysicsPartSpawner_Cubes.SpawnProbability` 0.8 _output_get)
  (`KismetSystemLibrary.Delay` 5.0)
  (`GameplayStatics.PlaySound2D` "/Game/Audio/Props/Halleluia/SC_STGrenade_Explo.SC_STGrenade_Explo" 1.0 1.0 0.0 null null)
  (`GameplayStatics.PlaySound2D` "/Game/Audio/Props/Dirt_layer/SC_Dirt_Explo.SC_Dirt_Explo" 1.0 1.0 0.0 null null)
  (bind _asbp_cam_player (cast `/Game/Nous/BP_CamPlayer` (`GameplayStatics.GetPlayerPawn` 0)))
  (`/Game/Nous/BP_CamPlayer.CamShake` _asbp_cam_player "/Game/Nous/ShakeSte.ShakeSte_C" (`self.K2_GetActorLocation`))
  (`VoxelSphereTools.RemoveSphere` (`self.World`) _returnvalue _returnvalue_2)
  (`|ExecutionSequence`
    (:`then_0`
      ;[1 1 1] Spawn some cubes inside the removed sphere
      (for _ (range 2501)
        ;;[1 1 1] Need to cache the result
        ;; else random will be different
        (bind _output_get_2 (set `self.RandomPosition` (+ _returnvalue (* (`KismetMathLibrary.RandomUnitVector`) (* _returnvalue_2 (`KismetMathLibrary.MultiplyMultiply_FloatFloat` (`KismetMathLibrary.RandomFloat`) 0.333333))))))
        (bind _returnvalue_5 (`VoxelWorld.GlobalToLocal` _world _output_get_2 "RoundToNearest"))
        ;;[1 1 1] Check if the voxel is full
        (bind _value (`VoxelDataTools.GetValue` _world _returnvalue_5))
        (if (<= _value 0.0)
          (bind _returnvalue_6 (`|SpawnActorFromClass` "/Script/Engine.StaticMeshActor" (`KismetMathLibrary.MakeTransform` (`self.RandomPosition`) (struct) (`KismetMathLibrary.Conv_DoubleToVector` (/ (`VoxelWorld.VoxelSize` _world) 100.0))) "Undefined" "OverrideRootScale" null null))
          (`StaticMeshActor.SetMobility` _returnvalue_6 "Movable")
          (`self.SetLifeSpan` _returnvalue_6 5.0)
          (bind _staticmeshcomponent (`StaticMeshActor.StaticMeshComponent` _returnvalue_6))
          (`StaticMeshComponent.SetStaticMesh` _staticmeshcomponent "/Engine/BasicShapes/Cube.Cube")
          (`PrimitiveComponent.SetSimulatePhysics` _staticmeshcomponent true)
          (`PrimitiveComponent.SetCollisionResponseToChannel` _staticmeshcomponent "ECC_Pawn" "ECR_Ignore")
          (`PrimitiveComponent.SetCollisionResponseToChannel` _staticmeshcomponent "ECC_Visibility" "ECR_Ignore")
          (bind _material (`VoxelDataTools.GetMaterial` _world _returnvalue_5))
          (bind _returnvalue_7 (`KismetMaterialLibrary.CreateDynamicMaterialInstance` "/Voxel/Examples/Materials/RGB/M_VoxelMaterial_Colors_Parameter.M_VoxelMaterial_Colors_Parameter"))
          (`MaterialInstanceDynamic.SetVectorParameterValue` _returnvalue_7 "VertexColor" (`VoxelBlueprintLibrary.GetColor` _material))
          (`PrimitiveComponent.SetMaterial` _staticmeshcomponent 0 _returnvalue_7))))
    (:`then_1`
      ;[1 1 1] Voxel physics
      (bind _results (`VoxelPhysicsTools.ApplyVoxelPhysics` _world_2 (`VoxelBlueprintLibrary.MakeIntBoxFromGlobalPositionAndRadius` _world_2 _returnvalue 400.0) (`self.NewVar`)))
      (for _array_element _results
        (bind _asvoxel_physics_part_spawner_result_cubes (cast `VoxelPhysicsPartSpawnerResult_Cubes` _array_element))
        (for _array_element_2 (`VoxelPhysicsPartSpawnerResult_Cubes.Cubes` _asvoxel_physics_part_spawner_result_cubes)
          (`self.SetLifeSpan` _array_element_2 5.0)
          (bind _staticmeshcomponent_2 (`StaticMeshActor.StaticMeshComponent` _array_element_2))
          (`PrimitiveComponent.SetCollisionResponseToChannel` _staticmeshcomponent_2 "ECC_Pawn" "ECR_Ignore")
          (`PrimitiveComponent.SetCollisionResponseToChannel` _staticmeshcomponent_2 "ECC_Visibility" "ECR_Ignore"))))
    (:`then_2`
      (`self.K2_DestroyActor`)
      (`self.Explosion`))))

(event `self.Sphere1.OnComponentHit`
  (params (HitComponent :type "PrimitiveComponent Object Reference") (OtherActor :type "Actor Object Reference") (OtherComp :type "PrimitiveComponent Object Reference") (NormalImpulse :type "Vector Structure") (Hit :type "HitResult Structure (by ref)"))
  (cast `VoxelWorld` OtherActor)
  (`GameplayStatics.PlaySound2D` "/Game/Audio/Props/Halleluia/SC_STGrenade_Bond.SC_STGrenade_Bond" 1.0 1.0 0.0 null null))

(event `Explosion`
  (`NiagaraFunctionLibrary.SpawnSystemAtLocation` "/Game/Nous/Niagara/NS_SainteGrenade.NS_SainteGrenade" (`self.K2_GetActorLocation`))
  (bind _returnvalue (`AddComponent|NODE_AddSphereComponent-0`))
  (add `PrimitiveComponent.OnComponentBeginOverlap` _returnvalue (delegate `OnComponentBeginOverlap_Event`)))

(event `OnComponentBeginOverlap_Event`
  (params (OverlappedComponent :type "PrimitiveComponent Object Reference") (OtherActor :type "Actor Object Reference") (OtherComp :type "PrimitiveComponent Object Reference") (OtherBodyIndex :type Integer) (bFromSweep :type Boolean) (SweepResult :type "HitResult Structure (by ref)"))
  (if (`KismetSystemLibrary.DoesImplementInterface` OtherActor "/Game/Nous/BPI_Destructible.BPI_Destructible_C")
    (message `/Game/Nous/BPI_Destructible.DestroySelf` OtherActor)))

(fn `UserConstructionScript`)