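; Fragmentation bomb that bounces on voxel terrain, then explodes with sound and Niagara effects into five BP_FragmentationOnce actors.
; A retriggerable fuse starts at BeginPlay and restarts on each voxel hit, with a hit limit forcing detonation.
; The blast's sphere carving, colored cube debris and voxel physics follow a short Delay, but fragment spawning and DestroyActor run immediately, before that Delay completes.
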(event `self.ReceiveBeginPlay`
  (`self.ExplosionRetard`)
  (bind _returnvalue (`|GenericCreateObject` self "/Script/Voxel.VoxelPhysicsPartSpawner_Cubes"))
  (bind _output_get (set `self.NewVar` _returnvalue))
  (set `VoxelPhysicsPartSpawner_Cubes.Material` "/Voxel/Examples/Materials/RGB/M_VoxelMaterial_Colors_Parameter.M_VoxelMaterial_Colors_Parameter" _output_get)
  (set `VoxelPhysicsPartSpawner_Cubes.SpawnProbability` 0.2 _output_get))

(event `ExplodeAnyway`
  (bind (_returnvalue_location _returnvalue_rotation _returnvalue_scale) (`KismetMathLibrary.BreakTransform` (`self.GetTransform`)))
  (bind _returnvalue (`self.K2_GetActorLocation`))
  (bind _returnvalue_2 (`self.K2_GetActorLocation`))
  (bind _returnvalue_3 (`KismetMathLibrary.RandomFloatInRange` 1500.0 1800.0))
  (bind _as_voxel_world (`self.As Voxel World`))
  (bind _as_voxel_world_2 (`self.As Voxel World`))
  (set `self.IsExploding` true :!label _label)
  (`|ExecutionSequence`
    (:`then_0`
      (`GameplayStatics.PlaySoundAtLocation` "/Game/Audio/Props/Bomb/SC_Bomb_Explo.SC_Bomb_Explo" _returnvalue (struct) 1.0 1.0 0.0 null null null null)
      (`GameplayStatics.PlaySoundAtLocation` "/Game/Audio/Props/Dirt_layer/SC_Dirt_Explo.SC_Dirt_Explo" _returnvalue (struct) 1.0 1.0 0.0 null null null null)
      (`NiagaraFunctionLibrary.SpawnSystemAtLocation` "/Game/Nous/Niagara/NS_Dynamite.NS_Dynamite" _returnvalue)
      (`KismetSystemLibrary.Delay` 0.2)
      (`VoxelSphereTools.RemoveSphere` (`self.As Voxel World`) _returnvalue_2 _returnvalue_3)
      (`|ExecutionSequence`
        (:`then_0`
          ;[1 1 1] Spawn some cubes inside the removed sphere
          (for _ (range 1001)
            ;;[1 1 1] Need to cache the result
            ;; else random will be different
            (bind _output_get (set `self.RandomPosition` (+ _returnvalue_2 (* (`KismetMathLibrary.RandomUnitVector`) (* _returnvalue_3 (`KismetMathLibrary.MultiplyMultiply_FloatFloat` (`KismetMathLibrary.RandomFloat`) 0.333333))))))
            (bind _returnvalue_4 (`VoxelWorld.GlobalToLocal` _as_voxel_world _output_get "RoundToNearest"))
            ;;[1 1 1] Check if the voxel is full
            (bind _value (`VoxelDataTools.GetValue` _as_voxel_world _returnvalue_4))
            (if (<= _value 0.0)
              (bind _returnvalue_5 (`|SpawnActorFromClass` "/Script/Engine.StaticMeshActor" (`KismetMathLibrary.MakeTransform` (`self.RandomPosition`) (struct) (`KismetMathLibrary.Conv_DoubleToVector` (/ (`VoxelWorld.VoxelSize` _as_voxel_world) 100.0))) "Undefined" "OverrideRootScale" null null))
              (`StaticMeshActor.SetMobility` _returnvalue_5 "Movable")
              (`self.SetLifeSpan` _returnvalue_5 5.0)
              (bind _staticmeshcomponent (`StaticMeshActor.StaticMeshComponent` _returnvalue_5))
              (`StaticMeshComponent.SetStaticMesh` _staticmeshcomponent "/Engine/BasicShapes/Cube.Cube")
              (`PrimitiveComponent.SetSimulatePhysics` _staticmeshcomponent true)
              (`PrimitiveComponent.SetCollisionResponseToChannel` _staticmeshcomponent "ECC_Pawn" "ECR_Ignore")
              (`PrimitiveComponent.SetCollisionResponseToChannel` _staticmeshcomponent "ECC_Visibility" "ECR_Ignore")
              (bind _material (`VoxelDataTools.GetMaterial` _as_voxel_world _returnvalue_4))
              (bind _returnvalue_6 (`KismetMaterialLibrary.CreateDynamicMaterialInstance` "/Voxel/Examples/Materials/RGB/M_VoxelMaterial_Colors_Parameter.M_VoxelMaterial_Colors_Parameter"))
              (`MaterialInstanceDynamic.SetVectorParameterValue` _returnvalue_6 "VertexColor" (`VoxelBlueprintLibrary.GetColor` _material))
              (`PrimitiveComponent.SetMaterial` _staticmeshcomponent 0 _returnvalue_6))))
        (:`then_1`
          ;[1 1 1] Voxel physics
          (bind _results (`VoxelPhysicsTools.ApplyVoxelPhysics` _as_voxel_world_2 (`VoxelBlueprintLibrary.MakeIntBoxFromGlobalPositionAndRadius` _as_voxel_world_2 _returnvalue_2 400.0) (`self.NewVar`)))
          (for _array_element _results
            (bind _asvoxel_physics_part_spawner_result_cubes (cast `VoxelPhysicsPartSpawnerResult_Cubes` _array_element))
            (for _array_element_2 (`VoxelPhysicsPartSpawnerResult_Cubes.Cubes` _asvoxel_physics_part_spawner_result_cubes)
              (`self.SetLifeSpan` _array_element_2 5.0)
              (bind _staticmeshcomponent_2 (`StaticMeshActor.StaticMeshComponent` _array_element_2))
              (`PrimitiveComponent.SetCollisionResponseToChannel` _staticmeshcomponent_2 "ECC_Pawn" "ECR_Ignore")
              (`PrimitiveComponent.SetCollisionResponseToChannel` _staticmeshcomponent_2 "ECC_Visibility" "ECR_Ignore"))))))
    (:`then_1`
      (for _index (range 5)
        (`|SpawnActorFromClass` "/Game/Nous/BP_FragmentationOnce.BP_FragmentationOnce_C" (`KismetMathLibrary.MakeTransform` (+ _returnvalue_location (select `int` _index :`0` (0.0 50.0 0.0) :`1` (25.0 25.0 0.0) :`2` (50.0 0.0 0.0) :`3` (25.0 -25.0 0.0) :`4` (0.0 50.0 0.0) :!type "Vector Structure")) _returnvalue_rotation _returnvalue_scale) "Undefined" "OverrideRootScale" null null)))
    (:`then_2`
      (`self.K2_DestroyActor`))))

(event `ExplosionRetard`
  (set `self.IsExploding` false)
  (`KismetSystemLibrary.RetriggerableDelay` 2.0)
  (goto _label))

(event `self.Sphere1.OnComponentHit`
  (params (HitComponent :type "PrimitiveComponent Object Reference") (OtherActor :type "Actor Object Reference") (OtherComp :type "PrimitiveComponent Object Reference") (NormalImpulse :type "Vector Structure") (Hit :type "HitResult Structure (by ref)"))
  (cast `VoxelWorld` OtherActor)
  (if (not (`self.IsExploding`))
    (`GameplayStatics.PlaySoundAtLocation` "/Game/Audio/Props/Bomb/SC_Bomb_Bond.SC_Bomb_Bond" (`self.K2_GetActorLocation`) (struct) 1.0 1.0 0.0 null null null null)
    (`self.ExplosionRetard`)
    (bind _output_get (set `self.HitCount` (+ (`self.HitCount`) 1)))
    (if (>= _output_get (`self.HitToExplode`))
      (`self.ExplodeAnyway`))))

(fn `UserConstructionScript`)