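; BP_CamPlayer is the player camera pawn, used to look around and drop explosives into the scene.
; Enhanced Input moves it vertically and, while rotation is held, hides the cursor and yaws the spring arm within a clamped range.
; On possession it adds the mapping context and a UI widget that references the pawn.
; Clicks trace under the cursor, spawning the EnumType-selected grenade or dynamite where they hit BP_PlaneInvisible.
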(event `EnhancedInput|/Game/Nous/IA_AllowRotation`
  (params (ActionValue :type Boolean) (ElapsedSeconds :type "Float (double-precision)") (TriggeredSeconds :type "Float (double-precision)") (InputAction :type "InputAction Object Reference" :default "/Game/Nous/IA_AllowRotation.IA_AllowRotation"))
  ;[1 1 1] RotationControl
  (:`Started`
    (set `self.AllowRotation` true)
    (set `PlayerController.bShowMouseCursor` false (`GameplayStatics.GetPlayerController` 0)))
  (:`Completed`
    (set `self.AllowRotation` false)
    (set `PlayerController.bShowMouseCursor` true (`GameplayStatics.GetPlayerController` 0))))

(event `EnhancedInput|/Game/Nous/IA_Move`
  (params (ActionValue :type "Float (double-precision)") (ElapsedSeconds :type "Float (double-precision)") (TriggeredSeconds :type "Float (double-precision)") (InputAction :type "InputAction Object Reference" :default "/Game/Nous/IA_Move.IA_Move"))
  ;[1 1 1] HeightControl
  (:`Triggered`
    (`self.AddMovementInput` (0.0 0.0 1.0) ActionValue true)))

(event `EnhancedInput|/Game/Nous/IA_Turn`
  (params (ActionValue :type "Float (double-precision)") (ElapsedSeconds :type "Float (double-precision)") (TriggeredSeconds :type "Float (double-precision)") (InputAction :type "InputAction Object Reference" :default "/Game/Nous/IA_Turn.IA_Turn"))
  (bind _maxrotationaxis (`self.MaxRotationAxis`))
  (bind _springarm (`self.SpringArm`))
  (bind (_relativerotation_roll _relativerotation_pitch _relativerotation_yaw) (`KismetMathLibrary.BreakRotator` (`SceneComponent.RelativeRotation` _springarm)))
  ;[1 1 1] RotationControl
  (:`Triggered`
    (if (`self.AllowRotation`)
      (`SceneComponent.K2_AddRelativeRotation` _springarm (`KismetMathLibrary.MakeRotator` 0.0 0.0 ActionValue) false false)
      (`SceneComponent.K2_SetRelativeRotation` _springarm (`KismetMathLibrary.MakeRotator` _relativerotation_roll _relativerotation_pitch (`KismetMathLibrary.FClamp` _relativerotation_yaw (* _maxrotationaxis -1.0) _maxrotationaxis)) false false))))

(event `self.ReceivePossessed`
  (params (NewController :type "Controller Object Reference"))
  (bind _returnvalue (`GameplayStatics.GetPlayerController` 0))
  (`/Engine/EditorBlueprintResources/StandardMacros.IsValid` _returnvalue
    (:`Is Valid`
      (`EnhancedInputSubsystemInterface.AddMappingContext` (pcsubsystem `EnhancedInputLocalPlayerSubsystem` _returnvalue) "/Game/Nous/IMC_Mapping.IMC_Mapping" 0 (struct))
      (set `PlayerController.bShowMouseCursor` true (`GameplayStatics.GetPlayerController` 0))
      (bind _returnvalue_2 (`|CreateWidget` "/Game/Nous/UI.UI_C"))
      (`UserWidget.AddToViewport` _returnvalue_2 0)
      (bind _output_get (set `self.UIREF` _returnvalue_2))
      (set `/Game/Nous/UI.playerpawn` self _output_get))))

(event `EnhancedInput|/Game/Nous/IA_Click`
  (params (ActionValue :type Boolean) (ElapsedSeconds :type "Float (double-precision)") (TriggeredSeconds :type "Float (double-precision)") (InputAction :type "InputAction Object Reference" :default "/Game/Nous/IA_Click.IA_Click"))
  (bind _hitresult (`PlayerController.GetHitResultUnderCursorForObjects` (`GameplayStatics.GetPlayerController` 0) (`|MakeArray` "ObjectTypeQuery7" :!type "EObjectTypeQuery Enum") true))
  (:`Started`
    (cast `/Game/Nous/BP_PlaneInvisible` (`.HitActor` (`GameplayStatics.BreakHitResult` _hitresult)))
    (`|SpawnActorFromClass` (select `/Game/Nous/ENUM_TypeGre` (`self.enum_type`) :`NewEnumerator0` "/Game/Nous/BP_Grenade.BP_Grenade_C" :`NewEnumerator1` "/Game/Nous/BP_Dynamite.BP_Dynamite_C" :`NewEnumerator2` "/Game/Nous/BP_SainteGrenade.BP_SainteGrenade_C" :`NewEnumerator3` "/Game/Nous/BP_Fragmentation.BP_Fragmentation_C" :!type "Actor Class Reference") (`KismetMathLibrary.MakeTransform` (`.ImpactPoint` (`GameplayStatics.BreakHitResult` _hitresult))) "Undefined" "OverrideRootScale")))

(fn `UserConstructionScript`)